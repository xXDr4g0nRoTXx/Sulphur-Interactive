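; Bear trap actor that catches the third-person player on overlap and holds them until they mash E.
; On overlap it disables movement, snaps the character to the box's X/Y, enables input, turns off box collision and plays a Timeline.
; E presses increment a counter; matching HowManyPresses restores walking and re-enables box collision after five seconds.
; The press counter is never reset.
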(event OnComponentBeginOverlap(Box)
  (params (OverlappedComponent :type Primitive%20Component%20Object%20Reference) (OtherActor :type Actor%20Object%20Reference) (OtherComp :type Primitive%20Component%20Object%20Reference) (OtherBodyIndex :type Integer) (bFromSweep :type Boolean) (SweepResult :type Hit%20Result%20Structure%20%28by%20ref%29))
  (bind _asbp_third_person_character (Utilities|Casting|CastToBP_ThirdPersonCharacter2 OtherActor))
  (CallFunction|CatchPlayer _asbp_third_person_character)
  (Input|EnableInput (Game|GetPlayerController 0) 0)
  (Collision|SetCollisionEnabled (Variables|Default|GetBox) "NoCollision")
  (Timeline|Timeline Play))

(event Custom|CatchPlayer
  (params (Character :type Character%20Object%20Reference))
  (bind _box (Variables|Default|GetBox))
  (bind _returnvalue (Transformation|GetWorldLocation _box))
  (Pawn|Components|CharacterMovement|DisableMovement (Variables|/Script/Engine.Character|GetCharacterMovement Character))
  (Transformation|SetActorLocation Character (Math|Vector|MakeVector (.x _returnvalue) (.y _returnvalue) (.z (Transformation|GetActorLocation Character))) false false))

(event Custom|Release
  (Pawn|Components|CharacterMovement|SetMovementMode (Variables|/Script/Engine.Character|GetCharacterMovement (stale OnComponentBeginOverlap(Box) _asbp_third_person_character)) "MOVE_Walking" 0)
  (Utilities|FlowControl|Delay 5.0)
  (Collision|SetCollisionEnabled (Variables|Default|GetBox) "QueryAndPhysics"))

(event EventBeginPlay)

(event Collision|EventActorBeginOverlap
  (params (OtherActor :type Actor%20Object%20Reference)))

(event EventTick
  (params (DeltaSeconds :type Float%20%28single-precision%29)))

(event Input|KeyboardEvents|E
  (params (Key :type Key%20Structure))
  (:Pressed
    (bind _result (Math|Integer|IncrementInt (Variables|Default|GetPresses))
      (:%20%20
        (if (== _result (Variables|Default|GetHowManyPresses))
          (CallFunction|Release))))))

(fn ConstructionScript)